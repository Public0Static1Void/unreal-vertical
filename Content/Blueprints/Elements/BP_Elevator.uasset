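; BP_Elevator is a signal-driven elevator actor that moves vertically between its starting height and a raised height.
; BeginPlay records the start Z and adds it to Height, turning that offset into an absolute target.
; The RecieveSignal event sets the Elevate flag, which selects the target height each Tick.
; Tick eases the actor toward that target with FInterpTo and a swept SetActorLocation, changing only Z.
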(event `self.ReceiveBeginPlay`
  (bind (_returnvalue_x _returnvalue_y _returnvalue_z) (`KismetMathLibrary.BreakVector` (`self.K2_GetActorLocation`)))
  (bind _output_get (set `self.startHeight` _returnvalue_z))
  (set `self.height` (+ _output_get (`self.height`))))

(event `/Game/Blueprints/BP_Interface.RecieveSignal`
  (params (isOn :type Boolean))
  (set `self.elevate` isOn))

(event `self.ReceiveTick`
  (params (DeltaSeconds :type "Float (single-precision)"))
  (bind (_returnvalue_x _returnvalue_y _returnvalue_z) (`KismetMathLibrary.BreakVector` (`self.K2_GetActorLocation`)))
  (if (`self.elevate`)
    (set `self.currHeight` (`self.height`))
    (else
      (set `self.currHeight` (`self.startHeight`))))
  (`self.K2_SetActorLocation` (`KismetMathLibrary.MakeVector` _returnvalue_x _returnvalue_y (`KismetMathLibrary.FInterpTo` _returnvalue_z (`self.currHeight`) DeltaSeconds 1.0)) true))

(fn `UserConstructionScript`)