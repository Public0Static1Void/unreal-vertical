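; BP_Button is a weight-triggered button that signals a list of target actors when a heavy enough object overlaps it.
; On begin and end overlap, it compares the mass of the other actor's StaticMeshComponent against ActivateMass.
; Qualifying overlaps send RecieveSignalMessage through BP_Interface to each implementing actor in ActorActivate, true on enter and false on exit.
; It keeps no overlap count, so any qualifying exit sends false.
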(event `self.ReceiveActorBeginOverlap`
  (params (OtherActor :type "Actor Object Reference"))
  (bind _returnvalue (`self.GetComponentByClass` OtherActor "/Script/Engine.StaticMeshComponent"))
  (`/Engine/EditorBlueprintResources/StandardMacros.IsValid` _returnvalue
    (:`Is Valid`
      (if (>= (`PrimitiveComponent.GetMass` _returnvalue) (`self.activateMass`))
        (for _array_element (`self.ActorActivate`)
          (if (`KismetSystemLibrary.DoesImplementInterface` _array_element "/Game/Blueprints/BP_Interface.BP_Interface_C")
            (message `/Game/Blueprints/BP_Interface.RecieveSignal` _array_element true)))))))

(event `self.ReceiveActorEndOverlap`
  (params (OtherActor :type "Actor Object Reference"))
  (bind _returnvalue (`self.GetComponentByClass` OtherActor "/Script/Engine.StaticMeshComponent"))
  (`/Engine/EditorBlueprintResources/StandardMacros.IsValid` _returnvalue
    (:`Is Valid`
      (if (>= (`PrimitiveComponent.GetMass` _returnvalue) (`self.activateMass`))
        (for _array_element (`self.ActorActivate`)
          (if (`KismetSystemLibrary.DoesImplementInterface` _array_element "/Game/Blueprints/BP_Interface.BP_Interface_C")
            (message `/Game/Blueprints/BP_Interface.RecieveSignal` _array_element false)))))))

(fn `UserConstructionScript`)