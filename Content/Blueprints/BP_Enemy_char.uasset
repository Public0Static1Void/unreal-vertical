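; Enemy character that spots the player through pawn sensing and drives its AI via blackboard keys for chasing state and returning to its last position.
; On sighting it stores its own location, and Tick switches it to return mode after about a second without seeing the player.
; When the ragdoll flag is set, Tick enables plane-constrained mesh physics, detaches the controller and pushes the mesh along a launch direction.
; Overlapping a void actor destroys it.
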(event `self.ReceiveTick`
  (params (DeltaSeconds :type "Float (single-precision)"))
  (bind _mesh (`self.Mesh`))
  (bind _as_bp_player_char (`self.As BP Player Char`))
  (bind _returnvalue (`AIBlueprintHelperLibrary.GetBlackboard` (`AIBlueprintHelperLibrary.GetAIController` self)))
  (if (`self.ragdoll`)
    (`PrimitiveComponent.SetSimulatePhysics` _mesh true)
    (`PrimitiveComponent.SetConstraintMode` _mesh "XYPlane")
    (`self.DetachFromControllerPendingDestroy`)
    (`SceneComponent.K2_AddWorldOffset` (`self.Mesh`) (`self.launchDir`) false true)
    (elif (`self.seenPlayer`)
      ;[1 1 1] Vuelve a la posición anterior
      (if (> (- (`KismetSystemLibrary.GetGameTimeInSeconds`) (`self.timeLastSeen`)) 1.0)
        (set `self.seenPlayer` false)
        (`BlackboardComponent.SetValueAsBool` _returnvalue "returnToLastPosition" true)
        (`BlackboardComponent.SetValueAsBool` _returnvalue "hasSeenPlayer" false))
      (else
        (`/Engine/EditorBlueprintResources/StandardMacros.IsValid` _as_bp_player_char
          (:`Is Valid`
            (if (<= (- (`KismetMathLibrary.VSize` (`self.GetNavAgentLocation` _as_bp_player_char)) (`KismetMathLibrary.VSize` (`self.lastPos`))) 0.1)
              (`BlackboardComponent.SetValueAsBool` _returnvalue "returnToLastPosition" false))))))))

(event `self.PawnSensing.OnSeePawn`
  (params (Pawn :type "Pawn Object Reference"))
  ;[0 0 0] Comprueba si ha visto al player
  (`/Engine/EditorBlueprintResources/StandardMacros.IsValid` Pawn
    (:`Is Valid`
      (bind _asbp_player_char (cast `/Game/Blueprints/BP_Player_char` Pawn))
      (set `self.As BP Player Char` _asbp_player_char)
      (`BlackboardComponent.SetValueAsBool` (`AIBlueprintHelperLibrary.GetBlackboard` (`AIBlueprintHelperLibrary.GetAIController` self)) "hasSeenPlayer" true)
      (if (not (`self.seenPlayer`))
        (set `self.seenPlayer` true)
        (set `self.lastPos` (`SceneComponent.K2_GetComponentLocation` (`self.CapsuleComponent`))))
      ;;[1 1 1] Tiempo visto x última vez
      (set `self.timeLastSeen` (`KismetSystemLibrary.GetGameTimeInSeconds`)))))

(event `self.ReceiveActorBeginOverlap`
  (params (OtherActor :type "Actor Object Reference"))
  (cast `/Game/Blueprints/Elements/BP_Void` OtherActor)
  (`self.K2_DestroyActor`))

(fn `UserConstructionScript`)